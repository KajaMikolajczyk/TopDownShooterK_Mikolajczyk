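; Game mode that endlessly spawns BP_Spider enemies during play.
; BeginPlay calls NewWave, which spawns one spider immediately and starts a looping timer that fires SpawnWave every few seconds.
; Each spawn picks a random TargetPoint in the level and, if valid, places one spider at its transform.
; CurrentWave increments with every spider spawned, so it acts as a spawn count; NewWave's own increment is unconnected.
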(event Custom|SpawnWave
  (CallFunction|SpawnSpooder))

(event EventBeginPlay
  (CallFunction|NewWave))

(event EventTick
  (params (DeltaSeconds :type Float%20%28single-precision%29)))

(fn ConstructionScript)

(fn NewWave
  (Utilities|Time|SetTimerbyFunctionName 0 "SpawnWave" 5.0 true)
  (CallFunction|SpawnSpooder))

(fn RSPoint
  (bind _outactors (Actor|GetAllActorsOfClass "/Script/Engine.TargetPoint"))
  (return (Utilities|Array|Get(acopy) _outactors (Math|Random|RandomIntegerinRange 0 (Utilities|Array|LastIndex _outactors)))))

(fn SpawnSpooder
  (bind _output (CallFunction|RSPoint))
  (Utilities|IsValid _output
    (:Is%20Valid
      (bind _result (Math|Integer|IncrementInt (Variables|Default|GetCurrentWave))
        (:%20%20
          (Variables|Default|SetCurrentWave _result)
          (Game|SpawnActorfromClass "/Game/Blueprints/AI/BP_Spider.BP_Spider_C" (Transformation|GetActorTransform _output) "Undefined" 0 0))))))