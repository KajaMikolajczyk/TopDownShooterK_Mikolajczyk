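; BP_Spider is an AI enemy that chases the player and attacks at close range.
; A looping AIMoveTo drives pursuit, while Tick pauses movement to play the attack montage when in range.
; DamagePlayer applies hit damage to the cached BP_Soldier_01 but is not called within this Blueprint.
; Incoming damage lowers clamped HP; at zero it credits the soldier's kill count, disables collision and destroys itself after a delay.
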(event EventBeginPlay
  (bind _asbp_soldier_01 (Utilities|Casting|CastToBP_Soldier_01 (Game|Player|GetPlayerPawn 0)))
  (Variables|Default|SetAs%20BP%20Soldier%2001 _asbp_soldier_01)
  (AI|AIMoveTo self "0, 0, 0" (Game|GetPlayerCharacter 0) 5.0 false :!label _label
    (:OnSuccess
      _)
    (:OnFail
      _))
  (Utilities|FlowControl|Delay 0.2)
  (goto _label))

(event Collision|EventActorBeginOverlap
  (params (OtherActor :type Actor%20Object%20Reference)))

(event EventTick
  (params (DeltaSeconds :type Float%20%28single-precision%29))
  ;[1 1 1] Spooder play attack
  (if (not (Variables|Default|GetDead))
    (if (and (CallFunction|IsAttackRange) (not (CallFunction|IsAttacking)))
      (Components|Activation|Deactivate (Variables|Character|GetCharacterMovement))
      (Animation|Montage|PlayMontage (Variables|Character|GetMesh) "/Game/Characters/Enemy_Great_Spider/Animations/SpooderAttack01.SpooderAttack01"
        (:OnCompleted
          (Components|Activation|Activate (Variables|Character|GetCharacterMovement) false))))))

(event Game|Damage|EventAnyDamage
  (params (Damage :type Float%20%28single-precision%29) (DamageType :type Damage%20Type%20Object%20Reference) (InstigatedBy :type Controller%20Object%20Reference) (DamageCauser :type Actor%20Object%20Reference))
  (bind _as_bp_soldier_01 (Variables|Default|GetAs%20BP%20Soldier%2001))
  ;[1 1 1] It doesn't matter if we turn to dust - Spooder
  (bind _output_get (CallFunction|DecreaseHP Damage))
  (if (== _output_get 0.0)
    (Variables|/Game/Blueprints/Pawns/BP_Soldier_01.BP_Soldier_01_C|SetKills _as_bp_soldier_01 (+ (Variables|/Game/Blueprints/Pawns/BP_Soldier_01.BP_Soldier_01_C|GetKills _as_bp_soldier_01) 1))
    (CallFunction|AIDead)
    (Utilities|FlowControl|Delay 2.0)
    (Actor|DestroyActor)))

(fn ConstructionScript)

(fn IsAttackRange
  (return (>= 155.0 (Transformation|GetDistanceTo (Game|GetPlayerCharacter 0)))))

(fn IsAttacking
  (return (Animation|Montage|MontageIsPlaying (Components|SkeletalMesh|GetAnimInstance (Variables|Character|GetMesh)) "/Game/Characters/Enemy_Great_Spider/Animations/SpooderAttack01.SpooderAttack01")))

(fn DamagePlayer
  (Game|Damage|ApplyDamage (Variables|Default|GetAs%20BP%20Soldier%2001) (Variables|Default|GetDamagePerHit) 0 0))

(fn DecreaseHP
  (params (Bambuko :type Float%20%28single-precision%29))
  (bind _output_get (Variables|Default|SetSpiderHP (Math|Float|Clamp(Float) (- (Variables|Default|GetSpiderHP) Bambuko) 0.0 1e+02)))
  (return _output_get))

(fn AIDead
  (Components|Movement|StopMovementImmediately (Variables|Character|GetCharacterMovement))
  (bind _output_get (Variables|Default|SetDead true))
  (Collision|SetActorEnableCollision false)
  (return _output_get))