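; Player soldier pawn with world-axis movement, mouse-driven aiming, an automatic rifle and a HUD widget.
; Each tick, mouse movement direction, not cursor position, sets an interpolated control yaw once its speed exceeds a deadzone.
; Firing runs muzzle effects, looping audio and a repeating timer for debug-drawn hitscan traces that apply damage along control rotation.
; Damage drains clamped health; zero sets Dead, which gates movement, aiming and starting fire.
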(event EventBeginPlay
  ;[1 1 1] HUD
  (bind _returnvalue (UserInterface|CreateWidget "/Game/UI/W_PlayerHud.W_PlayerHud_C" 0 self))
  (UserInterface|Viewport|AddtoViewport _returnvalue 0))

(event Collision|EventActorBeginOverlap
  (params (OtherActor :type Actor%20Object%20Reference)))

(event EventTick
  (params (DeltaSeconds :type Float%20%28single-precision%29))
  ;[1 1 1] Movement + camera
  (CallFunction|UpdatePlayerRotation))

(event Game|Damage|EventAnyDamage
  (params (Damage :type Float%20%28single-precision%29) (DamageType :type Damage%20Type%20Object%20Reference) (InstigatedBy :type Controller%20Object%20Reference) (DamageCauser :type Actor%20Object%20Reference))
  ;[1 1 1] Draining Soldiers life
  (bind _output_get (CallFunction|DecreaseHealth Damage))
  (if (<= _output_get 0.0)
    (Variables|Default|SetDead true)
    (Development|PrintString "Hello")))

(event Input|ActionEvents|InputActionFireWeapon
  (params (Key :type Key%20Structure :default "None"))
  ;[1 1 1] Bury me with my guns on
  (:Pressed
    (CallFunction|StartFiringWeapon)
    (CallFunction|WeaponTrace))
  (:Released
    (CallFunction|StopFiringWeapon)))

(event Input|AxisEvents|InputAxisMoveforwardback
  (params (AxisValue :type Float%20%28single-precision%29))
  ;[1 1 1] Movement + camera
  (if (CallFunction|IsAlive)
    (Pawn|Input|AddMovementInput "1.000000, 0, 0" AxisValue false)))

(event Input|AxisEvents|InputAxisMoveleftright
  (params (AxisValue :type Float%20%28single-precision%29))
  ;[1 1 1] Movement + camera
  (if (CallFunction|IsAlive)
    (Pawn|Input|AddMovementInput "0,1.000000, 0" AxisValue false)))

(fn ConstructionScript)

(fn GetMouseVelocity
  (bind _returnvalue (Game|GetPlayerController 0))
  (bind (_deltax _deltay) (Class|PlayerController|GetInputMouseDelta _returnvalue))
  (return (/ (Math|Vector2D|MakeVector2D _deltax _deltay) (Utilities|Time|GetWorldDeltaSeconds))))

(fn UpdatePlayerRotation
  (bind _returnvalue (Game|GetPlayerController 0))
  (bind _returnvalue_2 (CallFunction|GetMouseVelocity))
  (if (and (CallFunction|DeadzoneMouse) (CallFunction|IsAlive))
    (Pawn|SetControlRotation _returnvalue (Math|Interpolation|RInterpTo (Pawn|GetControlRotation _returnvalue :!class /Script/Engine.Controller) (Math|Rotator|MakeRotator 0.0 0.0 (Class|KismetMathLibrary|DegAtan2 (.x _returnvalue_2) (.y _returnvalue_2))) (Utilities|Time|GetWorldDeltaSeconds) (Variables|Default|GetInterp%20Speed)))))

(fn StartFiringWeapon
  (if (CallFunction|IsAlive)
    (Components|Activation|Activate (Variables|Default|GetP_AssaultRifle_MF) false)
    (bind _returnvalue (Audio|SpawnSound2D "/Game/Sounds/Weapon_AssaultRifle/Stereo/RandomFireloop.RandomFireloop" 1.0 1.0 0.0 0))
    (Variables|Default|SetWeaponFireSound _returnvalue)
    (CallFunction|WeaponTrace)
    (Utilities|Time|SetTimerbyFunctionName 0 "WeaponTrace" 0.1 true)
    (else
      (CallFunction|StopFiringWeapon))))

(fn StopFiringWeapon
  (bind _weaponfiresound (Variables|Default|GetWeaponFireSound))
  (Components|Activation|Deactivate (Variables|Default|GetP_AssaultRifle_MF))
  (Utilities|IsValid _weaponfiresound
    (:Is%20Valid
      (Audio|Components|Audio|Stop _weaponfiresound)
      (if (CallFunction|IsAlive)
        (Audio|SpawnSound2D "/Game/Sounds/Weapon_AssaultRifle/Stereo/GunfireEnd.GunfireEnd" 1.0 1.0 0.0 0)
        (Utilities|Time|ClearTimerbyFunctionName 0 "WeaponTrace")))))

(fn DeadzoneMouse
  (return (> (Math|Vector2D|Vector2DLength (CallFunction|GetMouseVelocity)) (Variables|Default|GetDeadMouseZoneVar))))

(fn DecreaseHealth
  (params (B :type Float%20%28single-precision%29))
  (bind _output_get (Variables|Default|SetHealth (Math|Float|Clamp(Float) (- (Variables|Default|GetHealth) B) 0.0 1e+02)))
  (return _output_get))

(fn IsAlive
  (return (not (Variables|Default|GetDead))))

(fn WeaponTrace
  (bind _outhit (Collision|LineTraceByChannel (CallFunction|GetWeaponTraceStartLocation) (CallFunction|GetWeaponTraceEndLocation) "TraceTypeQuery1" false 0 "ForDuration"))
  (if (.bBlockingHit (Collision|BreakHitResult _outhit))
    (Game|Damage|ApplyDamage (.HitActor (Collision|BreakHitResult _outhit)) 25.0 0 0)))

(fn GetWeaponTraceStartLocation
  (return (Transformation|GetSocketLocation (Variables|Default|GetRifle) "MuzzleFlashSocket")))

(fn GetWeaponTraceEndLocation
  (return (+ (CallFunction|GetWeaponTraceStartLocation) (* (Math|Vector|GetForwardVector (Pawn|GetControlRotation :!class /Script/Engine.Pawn)) (Variables|Default|GetWeaponRange)))))